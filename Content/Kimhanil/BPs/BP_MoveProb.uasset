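; BP_MoveProb is a prop actor that continuously drifts and spins its mesh through the world.
; Each tick it offsets the mesh transform by a move direction and rotation, scaled by their speeds and delta time, leaving scale unchanged.
; The construction script can roll a random move direction or rotation when the matching flag is set, then clears that flag so the value stays put.
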(event `self.ReceiveTick`
  (params (DeltaSeconds :type "Float (single-precision)"))
  (`SceneComponent.K2_AddWorldTransformKeepScale` (`self.Mesh`) (`KismetMathLibrary.MakeTransform` (* (`self.MoveDirection`) (* (`self.MoveSpeed`) DeltaSeconds)) (* (`self.RotateDirection`) (* DeltaSeconds (`self.RotateSpeed`))) (0.0 0.0 0.0)) false false))

(fn `UserConstructionScript`
  (if (`self.SetRandomRotDir`)
    (set `self.RotateDirection` (`KismetMathLibrary.RandomRotator` true))
    (set `self.SetRandomRotDir` false))
  (if (`self.SetRandomMoveDir`)
    (set `self.MoveDirection` (`KismetMathLibrary.RandomUnitVector`))
    (set `self.SetRandomMoveDir` false)))